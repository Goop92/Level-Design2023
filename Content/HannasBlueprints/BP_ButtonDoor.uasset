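; BP_ButtonDoor is an overlap-triggered button that opens doors sharing its DoorID.
; On BeginPlay its PointLight takes the unpressed color.
; Any actor overlap searches all BP_Door actors, calls OpenDoor on each matching ID, and switches the light to the pressed color.
; It has no end-overlap handling, so nothing in this Blueprint closes the doors or resets the light during play.
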(event `self.ReceiveBeginPlay`
  (`LightComponent.SetLightColor` (`self.PointLight`) (`self.ColorUnpressed`) true))

(event `self.ReceiveActorBeginOverlap`
  (params (OtherActor :type "Actor Object Reference"))
  (bind _outactors (`GameplayStatics.GetAllActorsOfClass` "/Game/HannasBlueprints/BP_Door.BP_Door_C"))
  (for _array_element _outactors
    (if (== (`/Game/HannasBlueprints/BP_Door.DoorID` _array_element) (`self.DoorID`))
      (`/Game/HannasBlueprints/BP_Door.OpenDoor` _array_element)))
  (`LightComponent.SetLightColor` (`self.PointLight`) (`self.ColorPressed`) true))

(fn `UserConstructionScript`)