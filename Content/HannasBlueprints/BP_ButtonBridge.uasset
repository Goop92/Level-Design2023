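; BP_ButtonBridge is a button actor that moves linked bridges whenever an actor begins overlapping it.
; On overlap it searches all BP_Bridge actors in the world and calls MoveBridge on those whose BridgeID is in its BridgeIDs list.
; Each overlap, with no filter on the overlapping actor, also toggles the Pressed state and switches the point light between pressed and unpressed colors.
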(event `self.ReceiveBeginPlay`
  (`LightComponent.SetLightColor` (`self.PointLight`) (`self.UnpressedColor`) true))

(event `self.ReceiveActorBeginOverlap`
  (params (OtherActor :type "Actor Object Reference"))
  (bind _outactors (`GameplayStatics.GetAllActorsOfClass` "/Game/HannasBlueprints/BP_Bridge.BP_Bridge_C"))
  (for _array_element _outactors
    (if (`KismetArrayLibrary.Array_Contains` (`self.BridgeIDs`) (`/Game/HannasBlueprints/BP_Bridge.BridgeID` _array_element))
      (`/Game/HannasBlueprints/BP_Bridge.MoveBridge` _array_element)))
  (if (`self.Pressed`)
    (set `self.Pressed` false)
    (`LightComponent.SetLightColor` (`self.PointLight`) (`self.UnpressedColor`) true)
    (else
      (set `self.Pressed` true)
      (`LightComponent.SetLightColor` (`self.PointLight`) (`self.PressedColor`) true))))

(fn `UserConstructionScript`)